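; BP_GrenadeProjectile is a grenade projectile that detonates on a fixed, short timer after BeginPlay rather than on impact.
; After the delay, the Explode custom event spawns the explosion particle effect at the actor's location.
; BeginPlay then applies radial damage within DamageRadius, credited to the instigator's controller, and destroys the actor.
; A debug sphere, drawn after the destroy call, shows the damage radius.
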(event Custom|Explode
  ;[1 1 1] 커스텀 이벤트로 폭발 하는것 과 시각적 효과와 폭발할 때 데미지를 준다
  (Effects|SpawnEmitteratLocation "/Game/StarterContent/Particles/P_Explosion.P_Explosion" (Transformation|GetActorLocation)))

(event EventBeginPlay
  (bind _returnvalue (Transformation|GetActorLocation))
  (Utilities|FlowControl|Delay 1.0)
  (CallFunction|Explode)
  (Game|Damage|ApplyRadialDamage 1e+02 _returnvalue (Variables|Default|GetDamageRadius) 0 0 self (Game|GetInstigatorController) false "ECC_Visibility")
  (Actor|DestroyActor)
  (Rendering|Debug|DrawDebugSphere _returnvalue (Variables|Default|GetDamageRadius) 12 "(R=1.000000,G=0.913555,B=0.000000,A=1.000000)" 1.0 1.0))

(fn ConstructionScript)